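; Player tank Blueprint that rides over terrain by moving and tilting itself kinematically, without sweeping for collisions.
; BeginPlay adds the tank input mapping context and caches its BP_GroundSensing components.
; Each Tick sums all sensor hits, divides by the grounded count, then aligns rotation to that normal and corrects height with an offset.
; Forward speed eases toward a target that nothing in this graph sets.
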(event `self.ReceiveBeginPlay`
  (`EnhancedInputSubsystemInterface.AddMappingContext` (pcsubsystem `EnhancedInputLocalPlayerSubsystem` (`GameplayStatics.GetPlayerController` 0)) "/Game/TheTankGame/inputs/IMC_Tank.IMC_Tank" 0 (struct))
  (set `self.GroundSensingArray` (`self.K2_GetComponentsByClass` "/Game/TheTankGame/BluePrint/BP_GroundSensing.BP_GroundSensing_C")))

(event `self.ReceiveTick`
  (params (DeltaSeconds :type "Float (single-precision)"))
  (bind _returnvalue (`GameplayStatics.GetWorldDeltaSeconds`))
  (bind (_returnvalue_x _returnvalue_y _returnvalue_z) (`KismetMathLibrary.BreakVector` (`self.K2_GetActorLocation`)))
  (bind _returnvalue_2 (`KismetMathLibrary.FInterpTo` (`self.CurrentForwardSpeed`) (`self.TargetForwardSpeed`) _returnvalue 2.0))
  (set `self.AvgNormal` (0.0 0.0 0.0))
  (set `self.AvgHeight` 0.0)
  (set `self.CountOnGround` 0)
  (for _array_element (`self.GroundSensingArray`)
    (set `self.AvgNormal` (+ (`/Game/TheTankGame/BluePrint/BP_GroundSensing.HitNormal` _array_element) (`self.AvgNormal`)))
    (bind (_hitlocation_x _hitlocation_y _hitlocation_z) (`KismetMathLibrary.BreakVector` (`/Game/TheTankGame/BluePrint/BP_GroundSensing.HitLocation` _array_element)))
    (set `self.AvgHeight` (+ _hitlocation_z (`self.AvgHeight`)))
    (if (`/Game/TheTankGame/BluePrint/BP_GroundSensing.onGround` _array_element)
      (`/Engine/EditorBlueprintResources/StandardMacros.IncrementInt` (`self.CountOnGround`))))
  (set `self.AvgNormal` (/ (`self.AvgNormal`) (`self.CountOnGround`)))
  (bind _output_get (set `self.AvgHeight` (/ (`self.AvgHeight`) (`self.CountOnGround`))))
  (set `self.DeltaZ` (- (+ _output_get (`self.HeightOffset`)) _returnvalue_z))
  (`self.K2_SetActorRotation` (`KismetMathLibrary.MakeRotFromZY` (`self.AvgNormal`) (`self.GetActorRightVector`)))
  (`self.K2_AddActorWorldOffset` (+ (* (`self.GetActorForwardVector`) _returnvalue_2 _returnvalue) (* (`self.GetActorUpVector`) (`self.DeltaZ`))))
  (set `self.CurrentForwardSpeed` _returnvalue_2))

(fn `UserConstructionScript`)