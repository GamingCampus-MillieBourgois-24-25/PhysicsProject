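; BP_Projectile is the projectile actor for the tank game, expiring after five seconds if nothing destroys it first.
; On a Sphere hit it attaches an auto-released, pooled BulletCollide effect to the struck component, oriented along the impact normal.
; It also spawns and triggers a scaled-up BP_MyMasterField at its location, then destroys both the field and itself after a short delay.
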(event `self.ReceiveBeginPlay`
  (`self.SetLifeSpan` 5.0))

(event `self.Sphere.OnComponentHit`
  (params (HitComponent :type "PrimitiveComponent Object Reference") (OtherActor :type "Actor Object Reference") (OtherComp :type "PrimitiveComponent Object Reference") (NormalImpulse :type "Vector Structure") (Hit :type "HitResult Structure (by ref)"))
  (bind (_bblockinghit _binitialoverlap _time _distance _location _impactpoint _normal _impactnormal _physmat _hitactor _hitcomponent) (`GameplayStatics.BreakHitResult` Hit))
  (if true
    (`NiagaraFunctionLibrary.SpawnSystemAttached` "/Game/TheTankGame/FX/BulletCollide.BulletCollide" _hitcomponent "None" (- _impactpoint (* _impactnormal (`self.10`))) (`KismetMathLibrary.Conv_VectorToRotator` _impactnormal) "KeepWorldPosition" true true "AutoRelease")
    (bind _returnvalue (`|SpawnActorFromClass` "/Game/02-Blueprints/Force/BP_MyMasterField.BP_MyMasterField_C" (`KismetMathLibrary.MakeTransform` (`self.K2_GetActorLocation`) (struct) (3.0 3.0 3.0)) "Undefined" "MultiplyWithRoot" null null))
    (set `/Engine/EditorResources/FieldNodes/FS_MasterField.ActivationType` "NewEnumerator4" _returnvalue)
    (`/Engine/EditorResources/FieldNodes/FS_MasterField.CE_Trigger` _returnvalue)
    (`KismetSystemLibrary.Delay` 0.2)
    (`self.K2_DestroyActor` _returnvalue)
    (`self.K2_DestroyActor` self)
    (else
      (`self.K2_DestroyActor`))))

(fn `UserConstructionScript`)